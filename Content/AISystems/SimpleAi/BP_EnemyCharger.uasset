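; BP_EnemyCharger is a melee enemy that chases the player from the start, driven by AI Move To on Tick.
; On reaching the player it stops and sweeps a claw box, whose overlap calls ChargerHit on the character.
; Arrow hits on head or body collision, debounced by DoOnce, deal different damage and award points through FirstPersonGameMode.
; At zero health it destroys itself and increments PointsToWin; PawnSensing is unused.
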(event `self.ClawAttackBox.OnComponentBeginOverlap`
  (params (OverlappedComponent :type "PrimitiveComponent Object Reference") (OtherActor :type "Actor Object Reference") (OtherComp :type "PrimitiveComponent Object Reference") (OtherBodyIndex :type Integer) (bFromSweep :type Boolean) (SweepResult :type "HitResult Structure (by ref)"))
  ;[1 1 1] Damage Player
  (bind _asfirst_person_character (cast `/Game/FirstPersonBP/Blueprints/FirstPersonCharacter` OtherActor))
  (`/Game/FirstPersonBP/Blueprints/FirstPersonCharacter.ChargerHit` _asfirst_person_character))

(event `Attack-Claw`
  ;[1 1 1] Claw Attack Temp
  (`SceneComponent.K2_SetRelativeLocation` (`self.AttackBox`) (80.0 -55.0 -4.0) true false)
  (`KismetSystemLibrary.Delay` 0.2)
  (`SceneComponent.K2_SetRelativeLocation` (`self.AttackBox`) (0.0 98.0 -4.0) true false))

(event `self.ReceiveTick`
  (params (DeltaSeconds :type "Float (single-precision)"))
  ;[1 1 1] Chase Player from Start
  (bind _asfirst_person_character (cast `/Game/FirstPersonBP/Blueprints/FirstPersonCharacter` (`GameplayStatics.GetPlayerCharacter` 0)))
  (`|AIMoveTo` self (0.0 0.0 0.0) _asfirst_person_character 90.0
    (:`OnSuccess`
      (`MovementComponent.StopMovementImmediately` (`self.CharacterMovement`))
      (`self.Attack-Claw`)
      (`KismetSystemLibrary.Delay` 0.5)
      (`|AIMoveTo` self (0.0 0.0 0.0) null 90.0))))

(event `self.PawnSensing.OnSeePawn`
  (params (Pawn :type "Pawn Object Reference"))
  ;[1 1 1] Seek Player
)

(event `self.Head.OnComponentHit`
  (params (HitComponent :type "PrimitiveComponent Object Reference") (OtherActor :type "Actor Object Reference") (OtherComp :type "PrimitiveComponent Object Reference") (NormalImpulse :type "Vector Structure") (Hit :type "HitResult Structure (by ref)"))
  ;[1 1 1] On Hit Head
  (cast `/Game/IBWP3DBowPackageFPS/Weapon/Arrows/BP_Arrow1` (stale `self.HeadCollision.OnComponentBeginOverlap` OtherActor) :!label _label)
  (`/Engine/EditorBlueprintResources/StandardMacros.DoOnce` false :!label _label_2
    (:`Completed`
      (`|ExecutionSequence`
        (:`then_0`
          (`KismetSystemLibrary.Delay` 0.1)
          (goto _label_2 :!via `Reset`))
        (:`then_1`
          (set `self.Current Enemy Health` (- (`self.Current Enemy Health`) 50))
          (if (<= (`self.Current Enemy Health`) 0)
            (`self.K2_DestroyActor`)
            (`self.KillPoints`))
          ;[1 1 1] AddPoints
          (bind _asfirst_person_game_mode (cast `/Game/FirstPersonBP/Blueprints/FirstPersonGameMode` (`GameplayStatics.GetGameMode`)))
          (`/Game/FirstPersonBP/Blueprints/FirstPersonGameMode.AddTargetPoints` _asfirst_person_game_mode (`self.HeadshotPoints`)))))))

(event `self.HeadCollision.OnComponentBeginOverlap`
  (params (OverlappedComponent :type "PrimitiveComponent Object Reference") (OtherActor :type "Actor Object Reference") (OtherComp :type "PrimitiveComponent Object Reference") (OtherBodyIndex :type Integer) (bFromSweep :type Boolean) (SweepResult :type "HitResult Structure (by ref)"))
  (goto _label))

(event `KillPoints`
  ;[1 1 1] Add Point for Kill
  (bind _asfirst_person_game_mode (cast `/Game/FirstPersonBP/Blueprints/FirstPersonGameMode` (`GameplayStatics.GetGameMode`)))
  (set `/Game/FirstPersonBP/Blueprints/FirstPersonGameMode.PointsToWin` (+ (`/Game/FirstPersonBP/Blueprints/FirstPersonGameMode.PointsToWin` _asfirst_person_game_mode) 1) _asfirst_person_game_mode))

(event `self.Body.OnComponentHit`
  (params (HitComponent :type "PrimitiveComponent Object Reference") (OtherActor :type "Actor Object Reference") (OtherComp :type "PrimitiveComponent Object Reference") (NormalImpulse :type "Vector Structure") (Hit :type "HitResult Structure (by ref)"))
  ;[1 1 1] On Hit Body
)

(event `self.BodyCollision.OnComponentBeginOverlap`
  (params (OverlappedComponent :type "PrimitiveComponent Object Reference") (OtherActor :type "Actor Object Reference") (OtherComp :type "PrimitiveComponent Object Reference") (OtherBodyIndex :type Integer) (bFromSweep :type Boolean) (SweepResult :type "HitResult Structure (by ref)"))
  ;[1 1 1] On Hit Body
  (cast `/Game/IBWP3DBowPackageFPS/Weapon/Arrows/BP_Arrow1` OtherActor)
  (`/Engine/EditorBlueprintResources/StandardMacros.DoOnce` false :!label _label_3
    (:`Completed`
      (`|ExecutionSequence`
        (:`then_0`
          (`KismetSystemLibrary.Delay` 0.1)
          (goto _label_3 :!via `Reset`))
        (:`then_1`
          (set `self.Current Enemy Health` (- (`self.Current Enemy Health`) 25))
          (if (<= (`self.Current Enemy Health`) 0)
            (`self.K2_DestroyActor`)
            (`self.KillPoints`))
          ;[1 1 1] AddPoints
          (bind _asfirst_person_game_mode (cast `/Game/FirstPersonBP/Blueprints/FirstPersonGameMode` (`GameplayStatics.GetGameMode`)))
          (`/Game/FirstPersonBP/Blueprints/FirstPersonGameMode.AddTargetPoints` _asfirst_person_game_mode (`self.TargetScore`)))))))

(fn `UserConstructionScript`)