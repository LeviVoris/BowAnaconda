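; BP_BossCharger is a boss enemy that chases the player on sight and takes damage from arrows.
; Pawn sensing stores the player for AI MoveTo, also reissued every Tick; ChargeAttack is an empty stub, its launch logic disconnected.
; Body and head overlaps use resetting DoOnce gates, with headshots dealing more damage, and award game-mode points.
; It creates a boss health HUD on BeginPlay; death adds a kill point and removes the HUD.
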(event `self.ReceiveTick`
  (params (DeltaSeconds :type "Float (single-precision)"))
  (`|AIMoveTo` self (0.0 0.0 0.0) (stale `self.PawnSensing.OnSeePawn` _asplayer_character) 180.0))

(event `self.PawnSensing.OnSeePawn`
  (params (Pawn :type "Pawn Object Reference"))
  ;[1 1 1] Seek Player
  (bind _asplayer_character (cast `/Game/FirstPersonBP/Blueprints/PlayerCharacter` Pawn))
  (`|AIMoveTo` self (0.0 0.0 0.0) _asplayer_character 180.0
    (:`OnSuccess`
      (`self.ChargeAttack`))))

(event `self.ReceiveBeginPlay`
  ;[1 1 1] Spawn Health Bar
  (bind _returnvalue (`|CreateWidget` "/Game/StarterContent/Widgets/BossHealthHUD.BossHealthHUD_C" (`GameplayStatics.GetPlayerController` 0)))
  (`UserWidget.AddToViewport` _returnvalue 0))

(event `ChargeAttack`
  ;[1 1 1] Test Charge Attack
)

(event `self.BodyCollision.OnComponentBeginOverlap`
  (params (OverlappedComponent :type "PrimitiveComponent Object Reference") (OtherActor :type "Actor Object Reference") (OtherComp :type "PrimitiveComponent Object Reference") (OtherBodyIndex :type Integer) (bFromSweep :type Boolean) (SweepResult :type "HitResult Structure (by ref)"))
  ;[1 1 1] On Hit Body
  (cast `/Game/IBWP3DBowPackageFPS/Weapon/Arrows/BP_Arrow1` OtherActor)
  (`/Engine/EditorBlueprintResources/StandardMacros.DoOnce` false :!label _label
    (:`Completed`
      (`|ExecutionSequence`
        (:`then_0`
          (`KismetSystemLibrary.Delay` 0.1)
          (goto _label :!via `Reset`))
        (:`then_1`
          (set `self.Current Enemy Health` (- (`self.Current Enemy Health`) 25))
          (if (<= (`self.Current Enemy Health`) 0)
            (`self.K2_DestroyActor`)
            (`self.BossKillPoints`))
          ;[1 1 1] AddPoints
          (bind _asfirst_person_game_mode (cast `/Game/FirstPersonBP/Blueprints/FirstPersonGameMode` (`GameplayStatics.GetGameMode`)))
          (`/Game/FirstPersonBP/Blueprints/FirstPersonGameMode.AddTargetPoints` _asfirst_person_game_mode (`self.TargetScore`)))))))

(event `self.Body.OnComponentHit`
  (params (HitComponent :type "PrimitiveComponent Object Reference") (OtherActor :type "Actor Object Reference") (OtherComp :type "PrimitiveComponent Object Reference") (NormalImpulse :type "Vector Structure") (Hit :type "HitResult Structure (by ref)"))
  ;[1 1 1] On Hit Body
)

(event `self.Head.OnComponentHit`
  (params (HitComponent :type "PrimitiveComponent Object Reference") (OtherActor :type "Actor Object Reference") (OtherComp :type "PrimitiveComponent Object Reference") (NormalImpulse :type "Vector Structure") (Hit :type "HitResult Structure (by ref)"))
  ;[1 1 1] On Hit Head
)

(event `BossKillPoints`
  ;[1 1 1] Add Point for Kill
  (bind _asfirst_person_game_mode (cast `/Game/FirstPersonBP/Blueprints/FirstPersonGameMode` (`GameplayStatics.GetGameMode`)))
  (set `/Game/FirstPersonBP/Blueprints/FirstPersonGameMode.BossKillPoint` (+ (`/Game/FirstPersonBP/Blueprints/FirstPersonGameMode.BossKillPoint` _asfirst_person_game_mode) 1) _asfirst_person_game_mode)
  ;[1 1 1] Remove Boss HealthBar
  (bind _foundwidgets (`WidgetBlueprintLibrary.GetAllWidgetsOfClass` "/Game/StarterContent/Widgets/BossHealthHUD.BossHealthHUD_C" false))
  (`Widget.RemoveFromParent` _foundwidgets))

(event `self.HeadCollsion.OnComponentBeginOverlap`
  (params (OverlappedComponent :type "PrimitiveComponent Object Reference") (OtherActor :type "Actor Object Reference") (OtherComp :type "PrimitiveComponent Object Reference") (OtherBodyIndex :type Integer) (bFromSweep :type Boolean) (SweepResult :type "HitResult Structure (by ref)"))
  ;[1 1 1] On Hit Head
  (cast `/Game/IBWP3DBowPackageFPS/Weapon/Arrows/BP_Arrow1` OtherActor)
  (`/Engine/EditorBlueprintResources/StandardMacros.DoOnce` false :!label _label_2
    (:`Completed`
      (`|ExecutionSequence`
        (:`then_0`
          (`KismetSystemLibrary.Delay` 0.1)
          (goto _label_2 :!via `Reset`))
        (:`then_1`
          (set `self.Current Enemy Health` (- (`self.Current Enemy Health`) 50))
          (if (<= (`self.Current Enemy Health`) 0)
            (`self.K2_DestroyActor`)
            (`self.BossKillPoints`))
          ;[1 1 1] AddPoints
          (bind _asfirst_person_game_mode (cast `/Game/FirstPersonBP/Blueprints/FirstPersonGameMode` (`GameplayStatics.GetGameMode`)))
          (`/Game/FirstPersonBP/Blueprints/FirstPersonGameMode.AddTargetPoints` _asfirst_person_game_mode (`self.HeadshotPoints`)))))))

(fn `UserConstructionScript`)