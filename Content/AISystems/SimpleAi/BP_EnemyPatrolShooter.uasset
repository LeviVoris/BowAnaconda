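; Enemy shooter that chases the player via a work-in-progress per-tick AI MoveTo.
; On seeing the player through PawnSensing, it turns to face them and launches an impulse-driven projectile, gated by a cooldown.
; Arrow hits on separate head and body colliders deal different damage and award score through FirstPersonGameMode, with kills incrementing its win counter.
; Random patrol points are set up on BeginPlay, but the timeline movement using them never runs.
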(event `self.ReceiveTick`
  (params (DeltaSeconds :type "Float (single-precision)"))
  ;[1 1 1] AI Move to - WIP
  (bind _asplayer_character (cast `/Game/FirstPersonBP/Blueprints/PlayerCharacter` (`GameplayStatics.GetPlayerCharacter` 0)))
  (`|AIMoveTo` self (0.0 0.0 0.0) _asplayer_character 400.0))

(event `self.PawnSensing.OnSeePawn`
  (params (Pawn :type "Pawn Object Reference"))
  ;[1 1 1] Face Player
  (bind _asplayer_character (cast `/Game/FirstPersonBP/Blueprints/PlayerCharacter` Pawn))
  (`|ExecutionSequence`
    (:`then_0`
      (`self.K2_SetActorRotation` (`KismetMathLibrary.FindLookAtRotation` (`self.K2_GetActorLocation`) (`self.K2_GetActorLocation` _asplayer_character))))
    (:`then_1`
      ;[1 1 1] SpawnProjectile
      (if (`self.SpawnProjectile`)
        (bind _returnvalue (`|SpawnActorFromClass` "/Game/AISystems/BP_EnemyProjectile.BP_EnemyProjectile_C" (`SceneComponent.K2_GetComponentToWorld` (`self.ProjectileSpawnLocation`)) "Undefined" "OverrideRootScale" null null))
        (`PrimitiveComponent.AddImpulse` (`/Game/AISystems/BP_EnemyProjectile.Cube` _returnvalue) (* (`SceneComponent.GetForwardVector` (`self.Body`)) (`self.ShootForce`)) "None" true)
        (set `self.SpawnProjectile` false)
        (`KismetSystemLibrary.Delay` 1.5)
        (set `self.SpawnProjectile` true)))))

(event `self.ReceiveBeginPlay`
  ;[1 1 1] Set Patrol Points
  (set `self.PatrolPoint` (`|MakeArray` (`SceneComponent.K2_GetComponentLocation` (`self.MovePosition1`)) (`SceneComponent.K2_GetComponentLocation` (`self.MovePosition2`)) (`SceneComponent.K2_GetComponentLocation` (`self.MovePosition3`))))
  (`self.GetRandomLocation`))

(event `self.Body Collision.OnComponentHit`
  (params (HitComponent :type "PrimitiveComponent Object Reference") (OtherActor :type "Actor Object Reference") (OtherComp :type "PrimitiveComponent Object Reference") (NormalImpulse :type "Vector Structure") (Hit :type "HitResult Structure (by ref)"))
  ;[1 1 1] On Hit Body
  (cast `/Game/IBWP3DBowPackageFPS/Weapon/Arrows/BP_Arrow1` OtherActor)
  (set `self.Current Enemy Health` (- (`self.Current Enemy Health`) 25))
  (if (<= (`self.Current Enemy Health`) 0)
    (`self.K2_DestroyActor`)
    (`self.KillPoints`))
  ;[1 1 1] AddPoints
  (bind _asfirst_person_game_mode (cast `/Game/FirstPersonBP/Blueprints/FirstPersonGameMode` (`GameplayStatics.GetGameMode`)))
  (`/Game/FirstPersonBP/Blueprints/FirstPersonGameMode.AddTargetPoints` _asfirst_person_game_mode (`self.TargetScore`)))

(event `KillPoints`
  ;[1 1 1] Add Point for Kill
  (bind _asfirst_person_game_mode (cast `/Game/FirstPersonBP/Blueprints/FirstPersonGameMode` (`GameplayStatics.GetGameMode`)))
  (set `/Game/FirstPersonBP/Blueprints/FirstPersonGameMode.PointsToWin` (+ (`/Game/FirstPersonBP/Blueprints/FirstPersonGameMode.PointsToWin` _asfirst_person_game_mode) 1) _asfirst_person_game_mode))

(event `self.HeadCollision.OnComponentHit`
  (params (HitComponent :type "PrimitiveComponent Object Reference") (OtherActor :type "Actor Object Reference") (OtherComp :type "PrimitiveComponent Object Reference") (NormalImpulse :type "Vector Structure") (Hit :type "HitResult Structure (by ref)"))
  ;[1 1 1] On Hit Head
  (cast `/Game/IBWP3DBowPackageFPS/Weapon/Arrows/BP_Arrow1` OtherActor)
  (set `self.Current Enemy Health` (- (`self.Current Enemy Health`) 50))
  (if (<= (`self.Current Enemy Health`) 0)
    (`self.K2_DestroyActor`)
    (`self.KillPoints`))
  ;[1 1 1] AddPoints
  (bind _asfirst_person_game_mode (cast `/Game/FirstPersonBP/Blueprints/FirstPersonGameMode` (`GameplayStatics.GetGameMode`)))
  (`/Game/FirstPersonBP/Blueprints/FirstPersonGameMode.AddTargetPoints` _asfirst_person_game_mode (`self.HeadShotPoints`)))

(fn `GetRandomLocation`
  (set `self.CurrentPatrolPoint` (`KismetMathLibrary.RandomInteger` (`KismetArrayLibrary.Array_Length` (`self.PatrolPoint`)))))

(fn `UserConstructionScript`)