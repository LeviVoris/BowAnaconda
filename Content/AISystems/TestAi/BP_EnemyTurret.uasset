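; Enemy turret AI that chases and shoots the player, awarding score and a win point through FirstPersonGameMode when damaged or killed.
; Tick turns it toward the player and issues AI MoveTo, while PawnSensing launches impulse-driven BP_EnemyProjectile shots gated by a delay flag.
; NormalArrow hits deal more damage to the head than the body.
; GroundThorns overlaps set a flag for damage over time, run by a Tick-triggered Delay loop.
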(event `self.ReceiveTick`
  (params (DeltaSeconds :type "Float (single-precision)"))
  (`|ExecutionSequence`
    (:`then_0`
      (`self.ChaseandShoot`))
    (:`then_1`
      (`self.ThornDamage`))))

(event `ChaseandShoot`
  ;[1 1 1] Track Player from Start/Move To
  (bind _asplayer_character (cast `/Game/FirstPersonBP/Blueprints/PlayerCharacter` (`GameplayStatics.GetPlayerCharacter` 0)))
  (`self.K2_SetActorRotation` (`KismetMathLibrary.FindLookAtRotation` (`self.K2_GetActorLocation`) (`self.K2_GetActorLocation` _asplayer_character)))
  (`|AIMoveTo` self (0.0 0.0 0.0) _asplayer_character 750.0))

(event `self.PawnSensing.OnSeePawn`
  (params (Pawn :type "Pawn Object Reference"))
  ;[1 1 1] Face Player
  (bind _asplayer_character (cast `/Game/FirstPersonBP/Blueprints/PlayerCharacter` Pawn))
  (`|ExecutionSequence`
    (:`then_0`
      (`self.K2_SetActorRotation` (`KismetMathLibrary.FindLookAtRotation` (`self.K2_GetActorLocation`) (`self.K2_GetActorLocation` _asplayer_character))))
    (:`then_1`
      ;[1 1 1] SpawnProjectile
      (if (`self.SpawnProjectile`)
        (bind _returnvalue (`|SpawnActorFromClass` "/Game/AISystems/BP_EnemyProjectile.BP_EnemyProjectile_C" (`SceneComponent.K2_GetComponentToWorld` (`self.ProjectileSpawnLocation`)) "Undefined" "OverrideRootScale" null null))
        (`PrimitiveComponent.AddImpulse` (`/Game/AISystems/BP_EnemyProjectile.Cube` _returnvalue) (* (`SceneComponent.GetForwardVector` (`self.Body`)) (`self.ShootForce`)) "None" true)
        (set `self.SpawnProjectile` false)
        (`KismetSystemLibrary.Delay` 1.5)
        (set `self.SpawnProjectile` true)))))

(event `self.BodyCollision.OnComponentHit`
  (params (HitComponent :type "PrimitiveComponent Object Reference") (OtherActor :type "Actor Object Reference") (OtherComp :type "PrimitiveComponent Object Reference") (NormalImpulse :type "Vector Structure") (Hit :type "HitResult Structure (by ref)"))
  ;[1 1 1] On Hit Body
  (cast `/Game/IBWP3DBowPackageFPS/Weapon/Arrows/NormalArrow` OtherActor)
  (set `self.Current Enemy Health` (- (`self.Current Enemy Health`) 25))
  (if (<= (`self.Current Enemy Health`) 0)
    (`self.K2_DestroyActor`)
    (`self.KillPoints`))
  (`self.AddBodyScorePoints`))

(event `KillPoints`
  ;[1 1 1] Add Point for Kill
  (bind _asfirst_person_game_mode (cast `/Game/FirstPersonBP/Blueprints/FirstPersonGameMode` (`GameplayStatics.GetGameMode`)))
  (set `/Game/FirstPersonBP/Blueprints/FirstPersonGameMode.PointsToWin` (+ (`/Game/FirstPersonBP/Blueprints/FirstPersonGameMode.PointsToWin` _asfirst_person_game_mode) 1) _asfirst_person_game_mode))

(event `self.HeadCollision.OnComponentHit`
  (params (HitComponent :type "PrimitiveComponent Object Reference") (OtherActor :type "Actor Object Reference") (OtherComp :type "PrimitiveComponent Object Reference") (NormalImpulse :type "Vector Structure") (Hit :type "HitResult Structure (by ref)"))
  ;[1 1 1] On Hit Head
  (cast `/Game/IBWP3DBowPackageFPS/Weapon/Arrows/NormalArrow` OtherActor)
  (set `self.Current Enemy Health` (- (`self.Current Enemy Health`) 50))
  (if (<= (`self.Current Enemy Health`) 0)
    (`self.K2_DestroyActor`)
    (`self.KillPoints`))
  (`self.AddHeadShotScorePoints`))

(event `AddBodyScorePoints`
  ;[1 1 1] AddBodyPoints
  (bind _asfirst_person_game_mode (cast `/Game/FirstPersonBP/Blueprints/FirstPersonGameMode` (`GameplayStatics.GetGameMode`)))
  (`/Game/FirstPersonBP/Blueprints/FirstPersonGameMode.AddScorePoints` _asfirst_person_game_mode (`self.BodyScorePoints`)))

(event `self.ThornDOTCollision.OnComponentBeginOverlap`
  (params (OverlappedComponent :type "PrimitiveComponent Object Reference") (OtherActor :type "Actor Object Reference") (OtherComp :type "PrimitiveComponent Object Reference") (OtherBodyIndex :type Integer) (bFromSweep :type Boolean) (SweepResult :type "HitResult Structure (by ref)"))
  ;[1 1 1] Thorn Detection
  (cast `/Game/CustomBPs/Triggers/GroundThorns` OtherActor)
  (set `self.InThorns?` true))

(event `AddHeadShotScorePoints`
  ;[1 1 1] AddHeadShotPoints
  (bind _asfirst_person_game_mode (cast `/Game/FirstPersonBP/Blueprints/FirstPersonGameMode` (`GameplayStatics.GetGameMode`)))
  (`/Game/FirstPersonBP/Blueprints/FirstPersonGameMode.AddScorePoints` _asfirst_person_game_mode (`self.HeadShotPoints`)))

(event `self.ThornDOTCollision.OnComponentEndOverlap`
  (params (OverlappedComponent :type "PrimitiveComponent Object Reference") (OtherActor :type "Actor Object Reference") (OtherComp :type "PrimitiveComponent Object Reference") (OtherBodyIndex :type Integer))
  ;[1 1 1] Thorn Detection
  (cast `/Game/CustomBPs/Triggers/GroundThorns` OtherActor)
  (set `self.InThorns?` false))

(event `ThornDamage`
  ;[1 1 1] ThornDamage - DOT
  (`KismetSystemLibrary.Delay` 0.4 :!label _label)
  (`|ExecutionSequence`
    (:`then_0`
      (if (`self.InThorns?`)
        (set `self.Current Enemy Health` (- (`self.Current Enemy Health`) 10))
        (`self.AddBodyScorePoints`)
        (goto _label)))
    (:`then_1`
      (if (<= (`self.Current Enemy Health`) 0)
        (`self.K2_DestroyActor`)
        (`self.KillPoints`)
        (`self.AddBodyScorePoints`)))))

(fn `UserConstructionScript`)