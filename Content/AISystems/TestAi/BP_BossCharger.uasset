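; Boss enemy that chases the player via AI MoveTo on Tick and pawn sensing, with a health bar widget shown from BeginPlay.
; Arrow hits on body and head colliders deal different damage and award score through the game mode.
; Thorn overlap enables delay-looped damage over time, driven from Tick.
; Death destroys the boss, adds a kill point and removes the health bar; ChargeAttack is an empty stub with its launch logic disconnected.
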(event `self.ReceiveTick`
  (params (DeltaSeconds :type "Float (single-precision)"))
  ;[1 1 1] Tick
  (`|ExecutionSequence`
    (:`then_0`
      (`self.MoveTo`))
    (:`then_1`
      (`self.ThornDamage`))))

(event `MoveTo`
  ;[1 1 1] MoveTo
  (bind _asplayer_character (cast `/Game/FirstPersonBP/Blueprints/PlayerCharacter` (`GameplayStatics.GetPlayerCharacter` 0)))
  (`|AIMoveTo` self (0.0 0.0 0.0) _asplayer_character 180.0))

(event `self.PawnSensing.OnSeePawn`
  (params (Pawn :type "Pawn Object Reference"))
  ;[1 1 1] Seek Player
  (bind _asplayer_character (cast `/Game/FirstPersonBP/Blueprints/PlayerCharacter` Pawn))
  (`|AIMoveTo` self (0.0 0.0 0.0) _asplayer_character 180.0
    (:`OnSuccess`
      (`self.ChargeAttack`))))

(event `self.ReceiveBeginPlay`
  ;[1 1 1] Spawn Health Bar
  (bind _returnvalue (`|CreateWidget` "/Game/CustomBPs/Widgets/HUD/BossHealthHUD.BossHealthHUD_C" (`GameplayStatics.GetPlayerController` 0)))
  (`UserWidget.AddToViewport` _returnvalue 0))

(event `ChargeAttack`
  ;[1 1 1] Test Charge Attack
)

(event `self.BodyCollision.OnComponentHit`
  (params (HitComponent :type "PrimitiveComponent Object Reference") (OtherActor :type "Actor Object Reference") (OtherComp :type "PrimitiveComponent Object Reference") (NormalImpulse :type "Vector Structure") (Hit :type "HitResult Structure (by ref)"))
  ;[1 1 1] On Hit Body
  (cast `/Game/IBWP3DBowPackageFPS/Weapon/Arrows/NormalArrow` OtherActor)
  (set `self.Current Enemy Health` (- (`self.Current Enemy Health`) 25))
  (if (<= (`self.Current Enemy Health`) 0)
    (`self.K2_DestroyActor`)
    (`self.BossKillPoints`))
  (`self.AddBodyScorePoints`))

(event `BossKillPoints`
  ;[1 1 1] Add Point for Kill
  (bind _asfirst_person_game_mode (cast `/Game/FirstPersonBP/Blueprints/FirstPersonGameMode` (`GameplayStatics.GetGameMode`)))
  (set `/Game/FirstPersonBP/Blueprints/FirstPersonGameMode.BossKillPoint` (+ (`/Game/FirstPersonBP/Blueprints/FirstPersonGameMode.BossKillPoint` _asfirst_person_game_mode) 1) _asfirst_person_game_mode)
  ;[1 1 1] Remove Boss HealthBar
  (bind _foundwidgets (`WidgetBlueprintLibrary.GetAllWidgetsOfClass` "/Game/CustomBPs/Widgets/HUD/BossHealthHUD.BossHealthHUD_C" false))
  (`Widget.RemoveFromParent` _foundwidgets))

(event `self.HeadCollsion.OnComponentHit`
  (params (HitComponent :type "PrimitiveComponent Object Reference") (OtherActor :type "Actor Object Reference") (OtherComp :type "PrimitiveComponent Object Reference") (NormalImpulse :type "Vector Structure") (Hit :type "HitResult Structure (by ref)"))
  ;[1 1 1] On Hit Head
  (cast `/Game/IBWP3DBowPackageFPS/Weapon/Arrows/NormalArrow` OtherActor)
  (set `self.Current Enemy Health` (- (`self.Current Enemy Health`) 50))
  (if (<= (`self.Current Enemy Health`) 0)
    (`self.K2_DestroyActor`)
    (`self.BossKillPoints`))
  (`self.AddHeadShootScorePoints`))

(event `AddBodyScorePoints`
  ;[1 1 1] AddBodyPoints
  (bind _asfirst_person_game_mode (cast `/Game/FirstPersonBP/Blueprints/FirstPersonGameMode` (`GameplayStatics.GetGameMode`)))
  (`/Game/FirstPersonBP/Blueprints/FirstPersonGameMode.AddScorePoints` _asfirst_person_game_mode (`self.BodyScorePoints`)))

(event `self.ThornDOTCollision.OnComponentBeginOverlap`
  (params (OverlappedComponent :type "PrimitiveComponent Object Reference") (OtherActor :type "Actor Object Reference") (OtherComp :type "PrimitiveComponent Object Reference") (OtherBodyIndex :type Integer) (bFromSweep :type Boolean) (SweepResult :type "HitResult Structure (by ref)"))
  ;[1 1 1] Thorn Detection
  (cast `/Game/CustomBPs/Triggers/GroundThorns` OtherActor)
  (set `self.InThorns?` true))

(event `AddHeadShootScorePoints`
  ;[1 1 1] AddHeadShotPoints
  (bind _asfirst_person_game_mode (cast `/Game/FirstPersonBP/Blueprints/FirstPersonGameMode` (`GameplayStatics.GetGameMode`)))
  (`/Game/FirstPersonBP/Blueprints/FirstPersonGameMode.AddScorePoints` _asfirst_person_game_mode (`self.HeadshotPoints`)))

(event `self.ThornDOTCollision.OnComponentEndOverlap`
  (params (OverlappedComponent :type "PrimitiveComponent Object Reference") (OtherActor :type "Actor Object Reference") (OtherComp :type "PrimitiveComponent Object Reference") (OtherBodyIndex :type Integer))
  ;[1 1 1] Thorn Detection
  (cast `/Game/CustomBPs/Triggers/GroundThorns` OtherActor)
  (set `self.InThorns?` false))

(event `ThornDamage`
  ;[1 1 1] ThornDamage - DOT
  (`KismetSystemLibrary.Delay` 0.4 :!label _label)
  (`|ExecutionSequence`
    (:`then_0`
      (if (`self.InThorns?`)
        (set `self.Current Enemy Health` (- (`self.Current Enemy Health`) 10))
        (`self.AddBodyScorePoints`)
        (goto _label)))
    (:`then_1`
      (if (<= (`self.Current Enemy Health`) 0)
        (`self.K2_DestroyActor`)
        (`self.BossKillPoints`)
        (`self.AddBodyScorePoints`)))))

(fn `UserConstructionScript`)