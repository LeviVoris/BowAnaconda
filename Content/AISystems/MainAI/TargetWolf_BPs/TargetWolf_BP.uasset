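; TargetWolf_BP is a wolf enemy that chases the player, bites in range and awards points when shot or killed.
; Tick drives AIMoveTo pursuit, delayed bites with pauses, and thorn damage over time, using flags and latent delays; sight-based seeking is unwired.
; Normal arrow hits deal body or heavier headshot damage and add score through FirstPersonGameMode.
; Death counts toward PointsToWin, ragdolls the wolf and destroys it with a poof effect.
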(event `self.ReceiveBeginPlay`
  ;[1 1 1] SpawnPoof
  (`NiagaraFunctionLibrary.SpawnSystemAtLocation` "/Game/AISystems/DeathPoof/Spawn_Poof.Spawn_Poof" (`SceneComponent.K2_GetComponentLocation` (`self.Mesh`))))

(event `Bite`
  ;[1 1 1] Bite
  (bind _asplayer_character (cast `/Game/FirstPersonBP/Blueprints/PlayerCharacter` (`GameplayStatics.GetPlayerCharacter` 0)))
  (if (`self.BiteRange`) :!label _label
    (`KismetSystemLibrary.Delay` 0.842)
    (`/Engine/EditorBlueprintResources/StandardMacros.DoOnce` false :!label _label_2
      (:`Completed`
        (`/Game/FirstPersonBP/Blueprints/PlayerCharacter.WolfBite` _asplayer_character)
        (set `self.Idle` true)
        (set `self.StopChase` true)
        (`KismetSystemLibrary.Delay` 1.0)
        (set `self.Idle` false)
        (set `self.StopChase` false)
        (`|ExecutionSequence`
          (:`then_0`
            (goto _label))
          (:`then_1`
            (goto _label_2 :!via `Reset`)))))))

(event `self.ReceiveTick`
  (params (DeltaSeconds :type "Float (single-precision)"))
  ;[1 1 1] Tick
  (`|ExecutionSequence`
    (:`then_0`
      (`self.Chase and Attack`))
    (:`then_1`
      (`self.ThornDamage`))
    (:`then_2`
      (`self.Bite`))))

(event `self.BiteHitBox.OnComponentBeginOverlap`
  (params (OverlappedComponent :type "PrimitiveComponent Object Reference") (OtherActor :type "Actor Object Reference") (OtherComp :type "PrimitiveComponent Object Reference") (OtherBodyIndex :type Integer) (bFromSweep :type Boolean) (SweepResult :type "HitResult Structure (by ref)"))
  ;[1 1 1] Bite
  (cast `/Game/FirstPersonBP/Blueprints/PlayerCharacter` OtherActor)
  (set `self.BiteRange` true))

(event `self.BiteHitBox.OnComponentEndOverlap`
  (params (OverlappedComponent :type "PrimitiveComponent Object Reference") (OtherActor :type "Actor Object Reference") (OtherComp :type "PrimitiveComponent Object Reference") (OtherBodyIndex :type Integer))
  ;[1 1 1] Bite
  (cast `/Game/FirstPersonBP/Blueprints/PlayerCharacter` OtherActor)
  (set `self.BiteRange` false))

(event `Chase and Attack`
  ;[1 1 1] Chase Player from Start
  (`|ExecutionSequence`
    (:`then_0`
      (`/Engine/EditorBlueprintResources/StandardMacros.DoOnce` false
        (:`Completed`
          (set `self.StopChase` true)
          (set `self.Idle` true)
          (`KismetSystemLibrary.Delay` 1.0)
          (set `self.Idle` false)
          (set `self.StopChase` false))))
    (:`then_1`
      (if (not (`self.StopChase`))
        (bind _asplayer_character (cast `/Game/FirstPersonBP/Blueprints/PlayerCharacter` (`GameplayStatics.GetPlayerCharacter` 0)))
        (`|AIMoveTo` self (0.0 0.0 0.0) _asplayer_character 120.0
          (:`OnSuccess`
            (set `self.AtPlayer` true))
          (:`OnFail`
            (set `self.AtPlayer` false)))))))

(event `self.PawnSensing.OnSeePawn`
  (params (Pawn :type "Pawn Object Reference"))
  ;[1 1 1] Seek Player
)

(event `self.Mesh.OnComponentHit`
  (params (HitComponent :type "PrimitiveComponent Object Reference") (OtherActor :type "Actor Object Reference") (OtherComp :type "PrimitiveComponent Object Reference") (NormalImpulse :type "Vector Structure") (Hit :type "HitResult Structure (by ref)"))
  ;[1 1 1] On Hit Body
  (cast `/Game/IBWP3DBowPackageFPS/Weapon/Arrows/NormalArrow` OtherActor)
  (set `self.CurrentEnemyHealth` (- (`self.CurrentEnemyHealth`) 40.0))
  (if (<= (`self.CurrentEnemyHealth`) 0.0)
    (`self.KillPoints`)
    (`self.AddBodyScorePoints`)
    (set `self.IsDead?` true)
    (`self.RagDoll`)
    (`KismetSystemLibrary.Delay` 2.0)
    (`NiagaraFunctionLibrary.SpawnSystemAtLocation` "/Game/AISystems/DeathPoof/P_DPoof.P_DPoof" (`SceneComponent.K2_GetComponentLocation` (`self.Mesh`)))
    (`self.K2_DestroyActor`)
    (else
      (`self.AddBodyScorePoints`))))

(event `self.HeadCollision.OnComponentHit`
  (params (HitComponent :type "PrimitiveComponent Object Reference") (OtherActor :type "Actor Object Reference") (OtherComp :type "PrimitiveComponent Object Reference") (NormalImpulse :type "Vector Structure") (Hit :type "HitResult Structure (by ref)"))
  ;[1 1 1] On Hit Head
  (cast `/Game/IBWP3DBowPackageFPS/Weapon/Arrows/NormalArrow` OtherActor)
  (set `self.CurrentEnemyHealth` (- (`self.CurrentEnemyHealth`) 50.0))
  (if (<= (`self.CurrentEnemyHealth`) 0.0)
    (`self.KillPoints`)
    (`self.AddHeadShotScorePoints`)
    (set `self.IsDead?` true)
    (`self.RagDoll`)
    (`KismetSystemLibrary.Delay` 2.0)
    (`NiagaraFunctionLibrary.SpawnSystemAtLocation` "/Game/AISystems/DeathPoof/P_DPoof.P_DPoof" (`SceneComponent.K2_GetComponentLocation` (`self.Mesh`)))
    (`self.K2_DestroyActor`)
    (else
      (`self.AddHeadShotScorePoints`))))

(event `self.ThornDOTCollision.OnComponentBeginOverlap`
  (params (OverlappedComponent :type "PrimitiveComponent Object Reference") (OtherActor :type "Actor Object Reference") (OtherComp :type "PrimitiveComponent Object Reference") (OtherBodyIndex :type Integer) (bFromSweep :type Boolean) (SweepResult :type "HitResult Structure (by ref)"))
  ;[1 1 1] Thorn Detection
  (cast `/Game/CustomBPs/Triggers/GroundThorns` OtherActor)
  (set `self.InThorns?` true))

(event `self.ThornDOTCollision.OnComponentEndOverlap`
  (params (OverlappedComponent :type "PrimitiveComponent Object Reference") (OtherActor :type "Actor Object Reference") (OtherComp :type "PrimitiveComponent Object Reference") (OtherBodyIndex :type Integer))
  ;[1 1 1] Thorn Detection
  (cast `/Game/CustomBPs/Triggers/GroundThorns` OtherActor)
  (set `self.InThorns?` false))

(event `ThornDamage`
  ;[1 1 1] ThornDamage - DOT
  (`KismetSystemLibrary.Delay` 0.4 :!label _label)
  (`|ExecutionSequence`
    (:`then_0`
      (if (`self.InThorns?`)
        (set `self.CurrentEnemyHealth` (- (`self.CurrentEnemyHealth`) 10.0))
        (`self.AddBodyScorePoints`)
        (goto _label)))
    (:`then_1`
      (if (<= (`self.CurrentEnemyHealth`) 0.0)
        (set `self.IsDead?` true)
        (`KismetSystemLibrary.Delay` 0.4)
        (`self.RagDoll`)
        (`self.KillPoints`)
        (`self.AddBodyScorePoints`)
        (`NiagaraFunctionLibrary.SpawnSystemAtLocation` "/Game/AISystems/DeathPoof/P_DPoof.P_DPoof" (`SceneComponent.K2_GetComponentLocation` (`self.Mesh`)))
        (`self.K2_DestroyActor`)))))

(event `KillPoints`
  ;[1 1 1] Add Point for Kill
  (bind _asfirst_person_game_mode (cast `/Game/FirstPersonBP/Blueprints/FirstPersonGameMode` (`GameplayStatics.GetGameMode`)))
  (set `/Game/FirstPersonBP/Blueprints/FirstPersonGameMode.PointsToWin` (+ (`/Game/FirstPersonBP/Blueprints/FirstPersonGameMode.PointsToWin` _asfirst_person_game_mode) 1) _asfirst_person_game_mode))

(event `AddBodyScorePoints`
  ;[1 1 1] AddBodyPoints
  (bind _asfirst_person_game_mode (cast `/Game/FirstPersonBP/Blueprints/FirstPersonGameMode` (`GameplayStatics.GetGameMode`)))
  (`/Game/FirstPersonBP/Blueprints/FirstPersonGameMode.AddScorePoints` _asfirst_person_game_mode (`self.Body Score Points`)))

(event `AddHeadShotScorePoints`
  ;[1 1 1] AddHeadShotPoints
  (bind _asfirst_person_game_mode (cast `/Game/FirstPersonBP/Blueprints/FirstPersonGameMode` (`GameplayStatics.GetGameMode`)))
  (`/Game/FirstPersonBP/Blueprints/FirstPersonGameMode.AddScorePoints` _asfirst_person_game_mode (`self.HeadshotScorePoints`)))

(fn `Ragdoll`
  (`PrimitiveComponent.SetSimulatePhysics` (`self.Mesh`) true)
  (`PrimitiveComponent.SetSimulatePhysics` (`self.HeadCollision`) true)
  (`PrimitiveComponent.SetSimulatePhysics` (`self.ThornDOTCollision`) true)
  (`CharacterMovementComponent.DisableMovement` (`self.CharacterMovement`))
  (set `self.IsDead?` false))

(fn `UserConstructionScript`)