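; HarpoonCan ranged enemy that chases the player and fires impulse-launched projectiles on a two-second cooldown.
; Tick drives AI MoveTo, whose result gates shooting, while PawnSensing turns the enemy toward the player and triggers shots.
; Arrow hits on body or head and a delay-based ground-thorn damage loop reduce health and award score.
; Death credits a win point to the game mode, ragdolls, then destroys the actor with a poof.
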(event `self.ReceiveBeginPlay`
  ;[1 1 1] SpawnPoof
  (`NiagaraFunctionLibrary.SpawnSystemAtLocation` "/Game/AISystems/DeathPoof/Spawn_Poof.Spawn_Poof" (`SceneComponent.K2_GetComponentLocation` (`self.Mesh`))))

(event `self.ReceiveTick`
  (params (DeltaSeconds :type "Float (single-precision)"))
  ;[1 1 1] Tick
  (`|ExecutionSequence`
    (:`then_0`
      (`self.ChaseandShoot`))
    (:`then_1`
      (`self.ThornDamage`))))

(event `ChaseandShoot`
  ;[1 1 1] Chase and Shoot
  (bind _asplayer_character (cast `/Game/FirstPersonBP/Blueprints/PlayerCharacter` (`GameplayStatics.GetPlayerCharacter` 0)))
  (`|AIMoveTo` self (0.0 0.0 0.0) _asplayer_character 900.0 true
    (:`OnSuccess`
      (set `self.AtPlayer` true))
    (:`OnFail`
      (set `self.AtPlayer` false))))

(event `KillPoints`
  ;[1 1 1] Add Point for Kill
  (bind _asfirst_person_game_mode (cast `/Game/FirstPersonBP/Blueprints/FirstPersonGameMode` (`GameplayStatics.GetGameMode`)))
  (set `/Game/FirstPersonBP/Blueprints/FirstPersonGameMode.PointsToWin` (+ (`/Game/FirstPersonBP/Blueprints/FirstPersonGameMode.PointsToWin` _asfirst_person_game_mode) 1) _asfirst_person_game_mode))

(event `self.PawnSensing.OnSeePawn`
  (params (Pawn :type "Pawn Object Reference"))
  ;[1 1 1] Face Player
  (bind _asplayer_character (cast `/Game/FirstPersonBP/Blueprints/PlayerCharacter` Pawn))
  (`|ExecutionSequence`
    (:`then_0`
      (`self.K2_SetActorRotation` (`KismetMathLibrary.FindLookAtRotation` (`self.K2_GetActorLocation`) (`self.K2_GetActorLocation` _asplayer_character))))
    (:`then_1`
      ;[1 1 1] SpawnProjectile
      (if (`self.SpawnProjectile`)
        (if (`self.AtPlayer`)
          (if (not (`self.IsDead`))
            (bind _returnvalue (`|SpawnActorFromClass` "/Game/AISystems/BP_EnemyProjectile.BP_EnemyProjectile_C" (`SceneComponent.K2_GetComponentToWorld` (`self.ProjectileSpawnLocation`)) "Undefined" "OverrideRootScale" null null))
            (`PrimitiveComponent.AddImpulse` (`/Game/AISystems/BP_EnemyProjectile.Cube` _returnvalue) (* (`SceneComponent.GetForwardVector` (`self.Mesh`)) (`self.ShootForce`)) "None" true)
            (`self.ShootingSound`)
            (set `self.SpawnProjectile` false)
            (`KismetSystemLibrary.Delay` 2.0)
            (set `self.SpawnProjectile` true)))))))

(event `AddBodyHitScorePoints`
  ;[1 1 1] AddBodyPoints
  (bind _asfirst_person_game_mode (cast `/Game/FirstPersonBP/Blueprints/FirstPersonGameMode` (`GameplayStatics.GetGameMode`)))
  (`/Game/FirstPersonBP/Blueprints/FirstPersonGameMode.AddScorePoints` _asfirst_person_game_mode (`self.BodyScorePoint`)))

(event `AddHeadShotScorePoints`
  ;[1 1 1] AddHeadPoints
  (bind _asfirst_person_game_mode (cast `/Game/FirstPersonBP/Blueprints/FirstPersonGameMode` (`GameplayStatics.GetGameMode`)))
  (`/Game/FirstPersonBP/Blueprints/FirstPersonGameMode.AddScorePoints` _asfirst_person_game_mode (`self.HeadShotPoints`)))

(event `ShootingSound`
  ;[1 1 1] ShootingSound
  (`GameplayStatics.SpawnSoundAttached` "/Game/Ultimate_Animal_Sounds/Wavs/Bird_Tweets/Bird_tweets_2.Bird_tweets_2" (`self.Mesh`) "None" (0.0 0.0 0.0) (struct) "KeepRelativeOffset" true 0.01 1.0 0.0 null null))

(event `self.Mesh.OnComponentHit`
  (params (HitComponent :type "PrimitiveComponent Object Reference") (OtherActor :type "Actor Object Reference") (OtherComp :type "PrimitiveComponent Object Reference") (NormalImpulse :type "Vector Structure") (Hit :type "HitResult Structure (by ref)"))
  ;[1 1 1] On Hit Body
  (cast `/Game/IBWP3DBowPackageFPS/Weapon/Arrows/NormalArrow` OtherActor)
  (set `self.CurrentEnemyHealth` (- (`self.CurrentEnemyHealth`) 40.0))
  (if (<= (`self.CurrentEnemyHealth`) 0.0)
    (`self.KillPoints`)
    (`self.AddBodyHitScorePoints`)
    (set `self.IsDead` true)
    (`KismetSystemLibrary.Delay` 0.4)
    (`self.RagDoll`)
    (`KismetSystemLibrary.Delay` 2.0)
    (`NiagaraFunctionLibrary.SpawnSystemAtLocation` "/Game/AISystems/DeathPoof/P_DPoof.P_DPoof" (`SceneComponent.K2_GetComponentLocation` (`self.Mesh`)))
    (`self.K2_DestroyActor`)
    (else
      (`self.AddBodyHitScorePoints`))))

(event `self.HeadCollision.OnComponentHit`
  (params (HitComponent :type "PrimitiveComponent Object Reference") (OtherActor :type "Actor Object Reference") (OtherComp :type "PrimitiveComponent Object Reference") (NormalImpulse :type "Vector Structure") (Hit :type "HitResult Structure (by ref)"))
  ;[1 1 1] On Hit Head
  (cast `/Game/IBWP3DBowPackageFPS/Weapon/Arrows/NormalArrow` OtherActor)
  (set `self.CurrentEnemyHealth` (- (`self.CurrentEnemyHealth`) 50.0))
  (if (<= (`self.CurrentEnemyHealth`) 0.0)
    (`self.KillPoints`)
    (`self.AddHeadShotScorePoints`)
    (set `self.IsDead` true)
    (`KismetSystemLibrary.Delay` 0.4)
    (`self.RagDoll`)
    (`KismetSystemLibrary.Delay` 2.0)
    (`NiagaraFunctionLibrary.SpawnSystemAtLocation` "/Game/AISystems/DeathPoof/P_DPoof.P_DPoof" (`SceneComponent.K2_GetComponentLocation` (`self.Mesh`)))
    (`self.K2_DestroyActor`)
    (else
      (`self.AddHeadShotScorePoints`))))

(event `self.Body Thorn Collision.OnComponentBeginOverlap`
  (params (OverlappedComponent :type "PrimitiveComponent Object Reference") (OtherActor :type "Actor Object Reference") (OtherComp :type "PrimitiveComponent Object Reference") (OtherBodyIndex :type Integer) (bFromSweep :type Boolean) (SweepResult :type "HitResult Structure (by ref)"))
  ;[1 1 1] Thorn Detection
  (cast `/Game/CustomBPs/Triggers/GroundThorns` OtherActor)
  (set `self.InThorns?` true))

(event `self.Body Thorn Collision.OnComponentEndOverlap`
  (params (OverlappedComponent :type "PrimitiveComponent Object Reference") (OtherActor :type "Actor Object Reference") (OtherComp :type "PrimitiveComponent Object Reference") (OtherBodyIndex :type Integer))
  ;[1 1 1] Thorn Detection
  (cast `/Game/CustomBPs/Triggers/GroundThorns` OtherActor)
  (set `self.InThorns?` false))

(event `ThornDamage`
  ;[1 1 1] ThornDamage - DOT
  (`KismetSystemLibrary.Delay` 0.4 :!label _label)
  (`|ExecutionSequence`
    (:`then_0`
      (if (`self.InThorns?`)
        (set `self.CurrentEnemyHealth` (- (`self.CurrentEnemyHealth`) 10.0))
        (`self.AddBodyHitScorePoints`)
        (goto _label)))
    (:`then_1`
      (if (<= (`self.CurrentEnemyHealth`) 0.0)
        (set `self.IsDead` true)
        (`KismetSystemLibrary.Delay` 0.4)
        (`self.RagDoll`)
        (`KismetSystemLibrary.Delay` 3.0)
        (`self.KillPoints`)
        (`self.AddBodyHitScorePoints`)
        (`NiagaraFunctionLibrary.SpawnSystemAtLocation` "/Game/AISystems/DeathPoof/P_DPoof.P_DPoof" (`SceneComponent.K2_GetComponentLocation` (`self.Mesh`)))
        (`self.K2_DestroyActor`)))))

(fn `RagDoll`
  (`PrimitiveComponent.SetSimulatePhysics` (`self.Mesh`) true)
  (`PrimitiveComponent.SetCollisionEnabled` (`self.Body Thorn Collision`) "NoCollision")
  (`PrimitiveComponent.SetCollisionEnabled` (`self.HeadCollision`) "NoCollision")
  (`CharacterMovementComponent.DisableMovement` (`self.CharacterMovement`))
  (set `self.IsDead` true))

(fn `UserConstructionScript`)